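; Player inventory component that stores item classes and amounts in a slot array sized by the player controller.
; AddItem fills partial stacks, then empty slots, recursing on overflow and returning any remainder.
; UseItem calls UseItem on an existing or newly spawned item actor, then decrements the slot.
; DropItem empties a slot and spawns a physics-simulated pickup at a short camera trace, while slot changes refresh the inventory grid widget.
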(event Custom|Initialize
  (bind _returnvalue (Game|GetPlayerController 0))
  (bind _ashg_player_controller (Utilities|Casting|CastToHG_PlayerController _returnvalue))
  (Utilities|Array|Resize (Variables|Default|GetInvetoryItemSlots) (Variables|/Game/Blueprints/Game/HG_PlayerController.HG_PlayerController_C|GetInventorySlots _ashg_player_controller))
  (Variables|Default|SetInventory%20Menu%20Reference (Variables|/Game/Blueprints/Game/HG_PlayerController.HG_PlayerController_C|GetInventoryMenuReference _ashg_player_controller))
  (bind _asl1_character (Utilities|Casting|CastToL1_Character (Game|GetPlayerCharacter 0)))
  (Variables|Default|SetPlayerReference _asl1_character))

(event EventBeginPlay
  (CallFunction|Initialize))

(fn AddItem
  (params (Item :type BP%20Inventory%20Item%20Master%20Class%20Reference) (Amount :type Integer))
  (bind (_success_ _index) (CallFunction|CheckforEmptyItemSlot))
  (bind (_success__2 _index_2) (CallFunction|CheckforEmptyItemSlot))
  (LocalVariables|SetLocalItem Item)
  (LocalVariables|SetLocalAmount Amount)
  (LocalVariables|SetLocalMaxStackAmount (.MaxStackAmount (Utilities|Struct|BreakS_ItemData (Utilities|GetClassDefaults (LocalVariables|GetLocalItem)))))
  (if (> (.MaxStackAmount (Utilities|Struct|BreakS_ItemData (Utilities|GetClassDefaults (LocalVariables|GetLocalItem)))) 1)
    (bind (_success__3 _index_3) (CallFunction|CheckforFreeSlot (LocalVariables|GetLocalItem)))
    (if _success__3
      (LocalVariables|SetLocalIndex _index_3)
      (if (> (+ (.Amount (CallFunction|CheckItemDataatIndex (LocalVariables|GetLocalIndex))) (LocalVariables|GetLocalAmount)) (LocalVariables|GetLocalMaxStackAmount))
        (LocalVariables|SetLocalAmount (- (+ (.Amount (CallFunction|CheckItemDataatIndex (LocalVariables|GetLocalIndex))) (LocalVariables|GetLocalAmount)) (LocalVariables|GetLocalMaxStackAmount)))
        (Utilities|Array|SetArrayElem (Variables|Default|GetInvetoryItemSlots) (LocalVariables|GetLocalIndex) (Utilities|Struct|MakeS_InventoryItems (LocalVariables|GetLocalItem) (LocalVariables|GetLocalMaxStackAmount)))
        (CallFunction|UpdateInventorySlots (LocalVariables|GetLocalIndex))
        (bind _remainder (CallFunction|AddItem (LocalVariables|GetLocalItem) (LocalVariables|GetLocalAmount)))
        (return true _remainder)
        (else
          (Utilities|Array|SetArrayElem (Variables|Default|GetInvetoryItemSlots) (LocalVariables|GetLocalIndex) (Utilities|Struct|MakeS_InventoryItems (LocalVariables|GetLocalItem) (+ (.Amount (CallFunction|CheckItemDataatIndex (LocalVariables|GetLocalIndex))) (LocalVariables|GetLocalAmount))))
          (CallFunction|UpdateInventorySlots (LocalVariables|GetLocalIndex))
          (return true 0)))
      (elif _success_
        (LocalVariables|SetLocalIndex _index)
        (if (> (LocalVariables|GetLocalAmount) (LocalVariables|GetLocalMaxStackAmount))
          (Utilities|Array|SetArrayElem (Variables|Default|GetInvetoryItemSlots) (LocalVariables|GetLocalIndex) (Utilities|Struct|MakeS_InventoryItems (LocalVariables|GetLocalItem) (LocalVariables|GetLocalMaxStackAmount)))
          (CallFunction|UpdateInventorySlots (LocalVariables|GetLocalIndex))
          (bind _remainder_2 (CallFunction|AddItem (LocalVariables|GetLocalItem) (- (LocalVariables|GetLocalAmount) (LocalVariables|GetLocalMaxStackAmount))))
          (return true _remainder_2)
          (else
            (Utilities|Array|SetArrayElem (Variables|Default|GetInvetoryItemSlots) (LocalVariables|GetLocalIndex) (Utilities|Struct|MakeS_InventoryItems (LocalVariables|GetLocalItem) (LocalVariables|GetLocalAmount)))
            (CallFunction|UpdateInventorySlots (LocalVariables|GetLocalIndex))
            (return true 0)))
        (else
          (return false (LocalVariables|GetLocalAmount)))))
    (elif _success__2
      (LocalVariables|SetLocalIndex _index_2)
      (Utilities|Array|SetArrayElem (Variables|Default|GetInvetoryItemSlots) (LocalVariables|GetLocalIndex) (Utilities|Struct|MakeS_InventoryItems (LocalVariables|GetLocalItem) 1))
      (CallFunction|UpdateInventorySlots (LocalVariables|GetLocalIndex))
      (if (> (- (LocalVariables|GetLocalAmount) 1) 0)
        (bind _remainder_3 (CallFunction|AddItem (LocalVariables|GetLocalItem) (- (LocalVariables|GetLocalAmount) 1)))
        (return true _remainder_3)
        (else
          (return true 0)))
      (else
        (Development|PrintString "No Free Slots")
        (return false (LocalVariables|GetLocalAmount))))))

(fn CheckforEmptyItemSlot
  (bind (_array_element _array_index) (Utilities|Array|ForEachLoopwithBreak (Variables|Default|GetInvetoryItemSlots) :!label _label)
    (:LoopBody
      (if (Utilities|IsValidClass (.item (Utilities|Struct|BreakS_InventoryItems _array_element)))
        (LocalVariables|SetLocalSuccess false)
        (else
          (LocalVariables|SetLocalSuccess true)
          (LocalVariables|SetLocalIndex _array_index)
          (goto _label Break))))
    (:Completed
      (return (LocalVariables|GetLocalSuccess) (LocalVariables|GetLocalIndex)))))

(fn CheckItemDataatIndex
  (params (Index :type Integer))
  (bind _invetoryitemslots (Variables|Default|GetInvetoryItemSlots))
  (bind _output (Utilities|Array|Get(acopy) _invetoryitemslots Index))
  (bind (_item _amount) (Utilities|Struct|BreakS_InventoryItems _output))
  (return _item _amount))

(fn UpdateInventorySlots
  (params (Index :type Integer))
  (Default|UpdateSlot (Utilities|Array|Get(acopy) (Variables|/Game/UMG/Inventory/WBP_InventoryGrid.WBP_InventoryGrid_C|GetSlot%20Arrays (Variables|/Game/UMG/Inventory/WBP_InventoryMenu.WBP_InventoryMenu_C|GetWBP_InventoryGrid (Variables|/Game/Blueprints/Game/HG_PlayerController.HG_PlayerController_C|GetInventoryMenuReference (.AsHG%20Player%20Controller (Utilities|Casting|CastToHG_PlayerController (Game|GetPlayerController 0)))))) Index)))

(fn CheckforFreeSlot
  (params (Item :type BP%20Inventory%20Item%20Master%20Class%20Reference))
  (bind (_array_element _array_index) (Utilities|Array|ForEachLoopwithBreak (Variables|Default|GetInvetoryItemSlots) :!label _label)
    (:LoopBody
      (if (and (== (.item (Utilities|Struct|BreakS_InventoryItems _array_element)) Item) (< (.Amount (Utilities|Struct|BreakS_InventoryItems _array_element)) (.maxstackamount (Utilities|GetClassDefaults Item))))
        (LocalVariables|SetLocalSucces true)
        (LocalVariables|SetLocalIndex _array_index)
        (goto _label Break)
        (else
          (LocalVariables|SetLocalSucces false))))
    (:Completed
      (return (LocalVariables|GetLocalSucces) (LocalVariables|GetLocalIndex)))))

(fn UseItem
  (params (Index :type Integer))
  (bind _output_get (LocalVariables|SetLocalIndex Index))
  (if (> (.Amount (CallFunction|CheckItemDataatIndex _output_get)) 0)
    (bind _returnvalue (Actor|GetActorOfClass (.Item (CallFunction|CheckItemDataatIndex _output_get))))
    (Utilities|IsValid _returnvalue
      (:Is%20Valid
        (Default|UseItem _returnvalue))
      (:Is%20Not%20Valid
        (bind _returnvalue_2 (Game|SpawnActorfromClass (.Item (CallFunction|CheckItemDataatIndex _output_get)) (Math|Transform|MakeTransform "0, 0, 0" "0, 0, 0" "1.000000,1.000000,1.000000") "Undefined" 0 0))
        (Default|UseItem _returnvalue_2)))
    (CallFunction|RemoveItem (LocalVariables|GetLocalIndex))
    (Default|CloseDropDownMenu (Variables|Default|GetInventory%20Menu%20Reference))))

(fn RemoveItem
  (params (Index :type Integer))
  (bind (_item _amount) (CallFunction|CheckItemDataatIndex Index))
  (if (> _amount 1)
    (Utilities|Array|SetArrayElem (Variables|Default|GetInvetoryItemSlots) Index (Utilities|Struct|MakeS_InventoryItems _item (- _amount 1)))
    (else
      (Utilities|Array|SetArrayElem (Variables|Default|GetInvetoryItemSlots) Index (Utilities|Struct|MakeS_InventoryItems 0 0))))
  (CallFunction|UpdateInventorySlots Index))

(fn DropItem
  (params (Index :type Integer))
  (bind _playerreference (Variables|Default|GetPlayerReference))
  (bind _camera (Variables|/Game/Blueprints/Game/Level1/L1_Character.L1_Character_C|GetCamera _playerreference))
  (bind _returnvalue (Transformation|GetWorldLocation _camera))
  (bind _output_get (LocalVariables|SetLocalIndex Index))
  (LocalVariables|SetLocalAmount (.Amount (CallFunction|CheckItemDataatIndex _output_get)))
  (LocalVariables|SetLocalClass (.Item (CallFunction|CheckItemDataatIndex _output_get)))
  (if (> (LocalVariables|GetLocalAmount) 0)
    (for _index (range 0 (- (LocalVariables|GetLocalAmount) 1))
      (CallFunction|RemoveItem (LocalVariables|GetLocalIndex)))
    (Default|CloseDropDownMenu (Variables|Default|GetInventory%20Menu%20Reference))
    (bind (_outhit _returnvalue_2) (Collision|LineTraceByChannel _returnvalue (+ _returnvalue (* (Math|Vector|GetForwardVector _camera) 2e+02)) "TraceTypeQuery1" false 0 "None"))
    (bind _returnvalue_3 (Game|SpawnActorfromClass (.PickupActor (Utilities|Struct|BreakS_ItemData (Utilities|GetClassDefaults (LocalVariables|GetLocalClass)))) (Math|Transform|MakeTransform (select _returnvalue_2 (.Location (Collision|BreakHitResult _outhit)) (.TraceEnd (Collision|BreakHitResult _outhit))) "0, 0, 0" "1.000000,1.000000,1.000000") "Undefined" 0 0))
    (bind _output_get_2 (Variables|/Game/Blueprints/Actors/Inventory/InventoryPickupActors/BP_PickupActor_Master.BP_PickupActor_Master_C|SetAmount _returnvalue_3 (LocalVariables|GetLocalAmount)))
    (Development|PrintString (Utilities|String|ToString(Integer) _output_get_2))
    (Physics|SetSimulatePhysics (Variables|/Game/Blueprints/Actors/Inventory/InventoryPickupActors/BP_PickupActor_Master.BP_PickupActor_Master_C|GetStaticMesh _returnvalue_3) true)))